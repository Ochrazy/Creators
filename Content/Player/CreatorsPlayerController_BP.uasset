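; Player controller that manages the HUD, a resource count and cursor-driven building placement.
; BeginPlay creates the HUD, whose resource text refreshes whenever AddResources changes the total.
; EnterBuildingMode spawns a collision-less building out of sight, which Tick snaps to the cursor's visibility trace.
; Click release or touch press drops it and restores collision; outside building mode, hitting no WorldDynamic object switches the HUD to the Build panel.
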(event `self.ReceiveBeginPlay`
  (`KismetSystemLibrary.Delay` 0.2)
  (bind _returnvalue (`|CreateWidget` "/Game/UI/HUD_Widget.HUD_Widget_C"))
  (bind _output_get (set `self.ResourcesWidget` _returnvalue))
  (`UserWidget.AddToViewport` _output_get 0)
  (bind _foundwidgets (`WidgetBlueprintLibrary.GetAllWidgetsOfClass` "/Game/UI/HUD_Widget.HUD_Widget_C"))
  (set `self.HUDWidget` (`|GetArrayItem` _foundwidgets))
  (`TextBlock.SetText` (`/Game/UI/HUD_Widget.Resources` (`self.HUDWidget`)) (`KismetTextLibrary.Conv_IntToText` (`self.NumResources`)) :!label _label))

(event `UpdateResourcesUI`
  (goto _label))

(event `self.ReceiveTick`
  (params (DeltaSeconds :type "Float (single-precision)"))
  ;[1 1 1] Building Mode - Follow Cursor
  (if (`self.bBuildingMode`)
    (`self.K2_SetActorLocation` (`self.BuildingToPlace`) (`.Location` (`GameplayStatics.BreakHitResult` (`self.GetHitResultUnderCursorByChannel` "TraceTypeQuery1"))) false false)))

(event `Key|LeftMouseButton`
  (params (Key :type "Key Structure" :default "AnyKey"))
  ;[1 1 1] Left Click
  (:`Released`
    (if (`self.bBuildingMode`) :!label _label_2
      (set `self.bBuildingMode` false)
      (`self.SetActorEnableCollision` (`self.BuildingToPlace`) true)
      (elif (not (`.ReturnValue` (`self.GetHitResultUnderCursorForObjects` (`|MakeArray` "ObjectTypeQuery2" :!type "EObjectTypeQuery Enum") false)))
        (`self.ShowBuildUI`)))))

(event `InputTouch`
  (params (Location :type "Vector Structure") (FingerIndex :type "ETouchIndex Enum"))
  ;[1 1 1] Left Click
  (:`Pressed`
    (goto _label_2)))

(fn `AddResources`
  (params (NumberOfResources :type Integer))
  (set `self.NumResources` (+ NumberOfResources (`self.NumResources`)))
  (`self.UpdateResourcesUI`))

(fn `EnterBuildingMode`
  (params (BuildingToBePlaced :type "Building Class Reference"))
  (bind _returnvalue (`|SpawnActorFromClass` BuildingToBePlaced (`KismetMathLibrary.MakeTransform` (0.0 0.0 -9000.0)) "AlwaysSpawn" "OverrideRootScale"))
  (bind _output_get (set `self.BuildingToPlace` _returnvalue))
  (`self.SetActorEnableCollision` _output_get false)
  (set `self.bBuildingMode` true))

(fn `ShowBuildingUI`
  (bind _hudwidget (`self.HUDWidget`))
  (`Widget.SetVisibility` (`/Game/UI/HUD_Widget.BuildPanel` _hudwidget) "Hidden")
  (`Widget.SetVisibility` (`/Game/UI/HUD_Widget.BuildingPanel` _hudwidget) "Visible"))

(fn `ShowBuildUI`
  (bind _hudwidget (`self.HUDWidget`))
  (`Widget.SetVisibility` (`/Game/UI/HUD_Widget.BuildPanel` _hudwidget) "Visible")
  (`Widget.SetVisibility` (`/Game/UI/HUD_Widget.BuildingPanel` _hudwidget) "Hidden"))

(fn `UserConstructionScript`)