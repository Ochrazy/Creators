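; Behavior tree task that lets a Collector pawn gather resources from a mining spot.
; On execute, it casts the blackboard's nearest mining spot to a MiningResource, retrieves a fixed batch and adds it to the controlled Collector.
; It then sets the full-inventory blackboard flag when the Collector's total reaches capacity and finishes successfully.
; The task fails if the spot is not a MiningResource.
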(event `self.ReceiveExecute`
  (params (OwnerActor :type "Actor Object Reference"))
  (bind _asmining_resource (cast `MiningResource` (`BTFunctionLibrary.GetBlackboardValueAsActor` (`self.NearestMiningSpot`)))
    (:`then`
      (bind _returnvalue (`MiningResource.RetrieveResources` _asmining_resource 50))
      (bind _ascollector (cast `/Game/Blueprints/Collector` (`Controller.K2_GetPawn` (`AIBlueprintHelperLibrary.GetAIController` OwnerActor))))
      (`/Game/Blueprints/Collector.AddResources` _ascollector _returnvalue)
      (bind _numberofresources (`/Game/Blueprints/Collector.GetNumResources` _ascollector))
      (`BTFunctionLibrary.SetBlackboardValueAsBool` (`self.bMinerFullInventory`) (> _numberofresources 99))
      (`self.FinishExecute` true))
    (:`CastFailed`
      (`self.FinishExecute` false))))