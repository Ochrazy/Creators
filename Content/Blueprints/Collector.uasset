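; Collector is a resource-gathering actor that accumulates a resource count and hands it over to a base.
; DeliverResources adds the carried amount to both the first player's CreatorsPlayerController_BP and the assigned Base, then resets the count; nothing is delivered if the controller cast fails.
; SetNewBase stores the Base and writes it to the actor's AI Blackboard, exposing it to AI logic.
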(event `self.ReceiveBeginPlay`)

(fn `AddResources`
  (params (NumberOfResources :type Integer))
  (set `self.NumResources` (+ NumberOfResources (`self.NumResources`))))

(fn `DeliverResources`
  (bind _numresources (`self.NumResources`))
  (bind _ascreators_player_controller_bp (cast `/Game/Player/CreatorsPlayerController_BP` (`GameplayStatics.GetPlayerController` 0)))
  (`/Game/Player/CreatorsPlayerController_BP.AddResources` _ascreators_player_controller_bp _numresources)
  (`/Game/Buildings/CollectorBase.AddResources` (`self.Base`) _numresources)
  (set `self.NumResources` 0))

(fn `GetNumResources`
  (returns (NumberOfResources :type Integer))
  (return (`self.NumResources`)))

(fn `SetNewBase`
  (params (NewBase :type "/Game/Buildings/CollectorBase Object Reference"))
  (bind _output_get (set `self.Base` NewBase))
  (`BlackboardComponent.SetValueAsObject` (`AIBlueprintHelperLibrary.GetBlackboard` self) (`self.BaseBBKeyName`) _output_get))

(fn `UserConstructionScript`)